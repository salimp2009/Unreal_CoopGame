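; Grenade projectile Blueprint that explodes one second after BeginPlay, with the fuse outcome decided by the server.
; Explode runs only with authority, spawning an explosion emitter, applying full radial damage within DamageRadius credited to the instigator, then destroying the actor and drawing a debug sphere.
; Multi_PlayEffects is an empty, uncalled stub, so nothing here sends the emitter or sphere to remote clients.
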(event Custom|Explode
  (bind _returnvalue (Transformation|GetActorLocation))
  (Networking|SwitchHasAuthority
    (:Authority
      (Effects|SpawnEmitteratLocation "/Game/WeaponEffects/Explosion/P_Explosion.P_Explosion" _returnvalue)
      (Game|Damage|ApplyRadialDamage 1e+02 _returnvalue (Variables|Default|GetDamageRadius) "/Script/Engine.DamageType" 0 self (Game|GetInstigatorController) true "ECC_Visibility")
      (Actor|DestroyActor)
      (Rendering|Debug|DrawDebugSphere _returnvalue (Variables|Default|GetDamageRadius) 12 "(R=0.881048,G=1.000000,B=0.088914,A=1.000000)" 1.5 2.0))))

(event Custom|Multi_PlayEffects)

(event EventBeginPlay
  (Utilities|FlowControl|Delay 1.0)
  (Networking|SwitchHasAuthority
    (:Authority
      (CallFunction|Explode))))

(fn ConstructionScript)